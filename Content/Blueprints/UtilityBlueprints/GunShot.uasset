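; GunShot is an actor that plays ambient gunfire sounds at a repeating interval.
; On BeginPlay it starts a looping timer with a delay picked once at random between a few seconds, so the interval stays fixed per instance.
; Each tick of the timer randomly plays either a single shot or a quick three-shot burst by replaying its Audio component with short delays.
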(event `MultipleGunShots`
  (bind _audio (`self.Audio`))
  (`AudioComponent.Play` _audio 0.0)
  (`KismetSystemLibrary.Delay` 0.1)
  (`AudioComponent.Play` _audio 0.0)
  (`KismetSystemLibrary.Delay` 0.1)
  (`AudioComponent.Play` (`self.Audio`) 0.0))

(event `GunShot`
  (`AudioComponent.Play` (`self.Audio`) 0.0))

(event `RandomShot`
  (if (`KismetMathLibrary.RandomBool`)
    (`self.MultipleGunShots`)
    (else
      (`self.GunShot`))))

(event `self.ReceiveBeginPlay`
  (`KismetSystemLibrary.K2_SetTimerDelegate` (delegate `RandomShot`) (`KismetMathLibrary.RandomFloatInRange` 2.0 5.0) true))

(fn `UserConstructionScript`)